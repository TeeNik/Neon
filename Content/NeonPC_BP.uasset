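; NeonPC_BP is a player controller that manages an on-screen action menu for clicked actors.
; On BeginPlay it creates the ActionMenu widget, adds it to the viewport and keeps it hidden.
; ShowActionMenu projects the clicked actor's world location to screen space, offsets the widget slightly and makes it visible.
; A right mouse press calls HideActionMenu to hide it again.
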(event `self.ReceiveBeginPlay`
  (bind _returnvalue (`|CreateWidget` "/Game/ActionMenu.ActionMenu_C"))
  (bind _output_get (set `self.wActionWidget` _returnvalue))
  (`UserWidget.AddToViewport` _output_get 0)
  (`Widget.SetVisibility` _output_get "Hidden"))

(event `Key|RightMouseButton`
  (params (Key :type "Key Structure"))
  (:`Pressed`
    (`self.HideActionMenu`)))

(fn `HideActionMenu`
  (`Widget.SetVisibility` (`self.wActionWidget`) "Hidden"))

(fn `ShowActionMenu`
  (params (ClickedActor :type "Actor Object Reference"))
  (bind _wactionwidget (`self.wActionWidget`))
  (`UserWidget.SetPositionInViewport` _wactionwidget (- (`self.ProjectWorldLocationToScreen` (`self.K2_GetActorLocation` ClickedActor)) (25.0 25.0)) true)
  (`Widget.SetVisibility` _wactionwidget "Visible"))

(fn `UserConstructionScript`)