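; Game mode that builds a flat, square grid of GridBase_BP actors when play begins.
; A single loop over CellsInRow squared derives column and row from the index by modulo and integer division, spaced by SizeOfCell.
; Each cell always spawns regardless of collision, squashed on Z into a thin tile.
; An unconnected CellsInRow setter never runs, and the construction script is empty.
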(event `self.ReceiveBeginPlay`
  (bind _cellsinrow (`self.CellsInRow`))
  (bind _cellsinrow_2 (`self.CellsInRow`))
  (bind _sizeofcell (`self.SizeOfCell`))
  (for _index (range (* _cellsinrow _cellsinrow))
    (`|SpawnActorFromClass` "/Game/GridBase_BP.GridBase_BP_C" (`KismetMathLibrary.MakeTransform` (`KismetMathLibrary.MakeVector` (`KismetMathLibrary.Conv_IntToDouble` (* (mod _index _cellsinrow_2) _sizeofcell)) (`KismetMathLibrary.Conv_IntToDouble` (* (/ _index _cellsinrow_2) _sizeofcell))) (struct) (1.0 1.0 0.01)) "AlwaysSpawn" "OverrideRootScale" null null)))

(fn `UserConstructionScript`)